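; BP_Damage_Zone is a hazard zone that repeatedly damages an actor inside its sphere.
; Overlap begin adds a Niagara component to that actor and starts a one-second delay loop of hit sound and random damage until any overlap ends.
; Tick spawns the Damage_zone effect on the mesh every frame, spins it and offsets it along local Y, flipping direction on exact relative Z checks.
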(event OnComponentEndOverlap(Sphere)
  (params (OverlappedComponent :type Primitive%20Component%20Object%20Reference) (OtherActor :type Actor%20Object%20Reference) (OtherComp :type Primitive%20Component%20Object%20Reference) (OtherBodyIndex :type Integer))
  (Variables|Default|SetPlayer%20in false))

(event OnComponentBeginOverlap(Sphere)
  (params (OverlappedComponent :type Primitive%20Component%20Object%20Reference) (OtherActor :type Actor%20Object%20Reference) (OtherComp :type Primitive%20Component%20Object%20Reference) (OtherBodyIndex :type Integer) (bFromSweep :type Boolean) (SweepResult :type Hit%20Result%20Structure%20%28by%20ref%29))
  (Variables|Default|SetPlayer%20in true)
  (AddComponent|AddNiagaraComponent OtherActor false)
  (if (Variables|Default|GetPlayer%20in) :!label _label
    (Audio|PlaySound2D "/Game/Sound/SC_HitSound.SC_HitSound" 1.0 1.0 0.0 0 0)
    (Game|Damage|ApplyDamage OtherActor (Math|Random|RandomFloatinRange 2.0 1e+01) 0 self)
    (Utilities|FlowControl|Delay 1.0)
    (goto _label)))

(event EventTick
  (params (DeltaSeconds :type Float%20%28single-precision%29))
  (Niagara|SpawnSystemAttached "/Game/Niagara/Damage_zone.Damage_zone" (Variables|Default|GetStaticMesh) "None" "0, 0, 0" "0, 0, 0" "KeepRelativeOffset" false)
  (Utilities|FlowControl|Sequence
    (:then_0
      (Transformation|AddLocalRotation (Variables|Default|GetStaticMesh) (Math|Rotator|MakeRotator 0.0 0.0 1.0) false false)
      (if (Variables|Default|GetUp_Down)
        (Transformation|AddLocalOffset (Variables|Default|GetStaticMesh) (Math|Vector|MakeVector 0.0 5.0 0.0) false false)
        (if (== (.z (Variables|/Script/Engine.SceneComponent|GetRelativeLocation (Variables|Default|GetStaticMesh))) 1.0)
          (Variables|Default|SetUp_Down false))
        (else
          (Transformation|AddLocalOffset (Variables|Default|GetStaticMesh) (Math|Vector|MakeVector 0.0 -5.0 0.0) false false)
          (if (== (.z (Variables|/Script/Engine.SceneComponent|GetRelativeLocation (Variables|Default|GetStaticMesh))) 0.0)
            (Variables|Default|SetUp_Down true)))))))

(fn ConstructionScript)
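; BP_Potion is a health pickup that spins and bobs between two heights on Tick, using fixed per-frame steps.
; When the player's BP_CustomTPS character overlaps its Box, it adds health, calls CheckHealth and plays potion and heal sounds.
; The same overlap destroys the actor, adds a Niagara component after the destroy call, and increments the Potion counter in BP_New_GameMode.
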(event OnComponentBeginOverlap(Box)
  (params (OverlappedComponent :type Primitive%20Component%20Object%20Reference) (OtherActor :type Actor%20Object%20Reference) (OtherComp :type Primitive%20Component%20Object%20Reference) (OtherBodyIndex :type Integer) (bFromSweep :type Boolean) (SweepResult :type Hit%20Result%20Structure%20%28by%20ref%29))
  (bind _returnvalue (Game|GetGameMode))
  (bind _asbp_new_game_mode (Utilities|Casting|CastToBP_New_GameMode _returnvalue))
  (Utilities|FlowControl|Sequence
    (:then_0
      (bind _asbp_custom_tps (Utilities|Casting|CastToBP_CustomTPS (Game|GetPlayerCharacter 0)))
      (if (== OtherActor _asbp_custom_tps)
        (Variables|/Game/Blueprints/BP_CustomTPS.BP_CustomTPS_C|SetHealth _asbp_custom_tps (+ (Variables|/Game/Blueprints/BP_CustomTPS.BP_CustomTPS_C|GetHealth _asbp_custom_tps) 2e+01))
        (Default|CheckHealth _asbp_custom_tps)
        (Audio|PlaySound2D "/Game/Sound/SC_Potion.SC_Potion" 1.0 1.0 0.0 0 0)
        (Actor|DestroyActor)
        (AddComponent|AddNiagaraComponent false)
        (Audio|PlaySound2D "/Game/Sound/Heal_Sound.Heal_Sound" 1.0 1.0 0.0 0 0)))
    (:then_1
      (if (== (.AsBP%20Custom%20TPS (Utilities|Casting|CastToBP_CustomTPS (Game|GetPlayerCharacter 0))) OtherActor)
        (Variables|/Game/Core/BP_New_GameMode.BP_New_GameMode_C|SetPotion _asbp_new_game_mode (+ (Variables|/Game/Core/BP_New_GameMode.BP_New_GameMode_C|GetPotion _asbp_new_game_mode) 1))))))

(event EventTick
  (params (DeltaSeconds :type Float%20%28single-precision%29))
  (Transformation|AddLocalRotation (Variables|Default|GetStaticMesh) (Math|Rotator|MakeRotator 0.0 0.0 1.0) false false)
  (if (Variables|Default|GetUp_Down)
    (Transformation|AddLocalOffset (Variables|Default|GetStaticMesh) (Math|Vector|MakeVector 0.0 0.0 1.0) false false)
    (if (== (.z (Variables|/Script/Engine.SceneComponent|GetRelativeLocation (Variables|Default|GetStaticMesh))) 5e+01)
      (Variables|Default|SetUp_Down false))
    (else
      (Transformation|AddLocalOffset (Variables|Default|GetStaticMesh) (Math|Vector|MakeVector 0.0 0.0 -1.0) false false)
      (if (== (.z (Variables|/Script/Engine.SceneComponent|GetRelativeLocation (Variables|Default|GetStaticMesh))) 0.0)
        (Variables|Default|SetUp_Down true)))))

(fn ConstructionScript)
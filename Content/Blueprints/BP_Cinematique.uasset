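; Trigger actor that plays the CinematiqueFix level sequence once, on the first actor overlap.
; It stops the sound manager's music, hides the BP_CustomTPS mesh and disables player input, then plays a 2D sound partway through.
; After a timed delay rather than a sequence-finished event, it restores input, mesh and music.
; IsPlaying is set on every overlap, ahead of the DoOnce, and cleared only when that single run ends.
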(event Collision|EventActorBeginOverlap
  (params (OtherActor :type Actor%20Object%20Reference))
  (bind _returnvalue (Game|Player|GetPlayerPawn 0))
  (bind _returnvalue_2 (Game|GetPlayerController 0))
  (Variables|Default|SetIsPlaying true)
  (Utilities|FlowControl|DoOnce false
    (:Completed
      (bind _returnvalue_3 (Actor|GetActorOfClass "/Game/Blueprints/BP_SoundManager.BP_SoundManager_C"))
      (Audio|Components|Audio|Stop (Variables|/Game/Blueprints/BP_SoundManager.BP_SoundManager_C|GetMusique _returnvalue_3))
      (bind _returnvalue_4 (Actor|GetActorOfClass "/Game/Blueprints/BP_CustomTPS.BP_CustomTPS_C"))
      (Rendering|SetVisibility (Variables|/Script/Engine.Character|GetMesh _returnvalue_4) false false)
      (Input|DisableInput _returnvalue _returnvalue_2)
      (bind _returnvalue_5 (Sequencer|Player|CreateLevelSequencePlayer "/Game/Cinematic/CinematiqueFix.CinematiqueFix"))
      (Sequencer|Player|Play _returnvalue_5 :!class /Script/MovieScene.MovieSceneSequencePlayer)
      (Utilities|FlowControl|Delay 5.0)
      (Audio|PlaySound2D "/Game/Sound/CHILL_DREAM_-_Gaming_Sound_Effect_HD_FREE_NO_Copyright.CHILL_DREAM_-_Gaming_Sound_Effect_HD_FREE_NO_Copyright" 3.0 1.0 0.0 0 0)
      (Utilities|FlowControl|Delay (Variables|Default|GetDurée%20Cinematime))
      (Input|EnableInput _returnvalue _returnvalue_2)
      (Rendering|SetVisibility (Variables|/Script/Engine.Character|GetMesh _returnvalue_4) true false)
      (Audio|Components|Audio|Play (Variables|/Game/Blueprints/BP_SoundManager.BP_SoundManager_C|GetMusique _returnvalue_3) 0.0)
      (Variables|Default|SetIsPlaying false))))

(fn ConstructionScript)
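; Pickup weapon actor whose static mesh is assigned from ItemModelPlaced in the construction script.
; On PickUp it plays the Shrink timeline, scaling the root from full size to zero, with a short delay and destroy chained from the timeline update.
; In parallel it casts the player character to BP_CustomTPS and sets its PossedeMass and HaveWeapon flags.
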(event EventPickUp
  (Utilities|FlowControl|Sequence
    (:then_0
      (bind _shrink (Timeline|Shrink Play)
        (:Update
          (Transformation|SetWorldScale3D (Variables|Default|GetDefaultSceneRoot) (Math|Conversions|ToVector(Float) (Math|Float|Lerp 1.0 0.0 _shrink)))
          (Utilities|FlowControl|Delay 0.4)
          (Actor|DestroyActor))))
    (:then_1
      (bind _asbp_custom_tps (Utilities|Casting|CastToBP_CustomTPS (Game|GetPlayerCharacter 0)))
      (Variables|/Game/Blueprints/BP_CustomTPS.BP_CustomTPS_C|SetPossede_Mass _asbp_custom_tps true)
      (Variables|/Game/Blueprints/BP_CustomTPS.BP_CustomTPS_C|SetHave_weapon _asbp_custom_tps true))))

(fn ConstructionScript
  (Components|StaticMesh|SetStaticMesh (Variables|Default|GetItem_Model) (Variables|Default|GetItem_Model_Placed)))